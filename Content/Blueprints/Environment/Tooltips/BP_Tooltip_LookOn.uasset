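; Tooltip actor, extending a parent tooltip Blueprint, whose text turns to face the player's camera while the character is inside its box.
; Overlap events call the parent to track the character, then set or clear a look-at flag.
; While that flag is set, Tick rotates the text component each frame toward the third-person character's follow camera using a look-at rotation.
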(event EventTick
  (params (DeltaSeconds :type Float%20%28single-precision%29))
  ;[1 1 1] Rotate the text tooltip towards the player's camera every frame
  (|CallParentFunction DeltaSeconds)
  (CallFunction|LookingatPlayerCamera))

(event EventActorBeginOverlap
  (params (OtherActor :type Actor%20Object%20Reference))
  ;[1 1 1] Call the parent method to track the intersection with the player character
  (|CallParentFunction OtherActor)
  (Variables|Default|GetCharacterInBox
    (:then
      (Variables|Default|SetIsLookAtPlayerCamera true))
    (:else)))

(event EventActorEndOverlap
  (params (OtherActor :type Actor%20Object%20Reference))
  ;[1 1 1] Call the parent method to track the termination of the intersection with the player character
  (|CallParentFunction OtherActor)
  (Variables|Default|SetIsLookAtPlayerCamera false))

(fn ConstructionScript
  (|CallParentFunction))

(fn LookingatPlayerCamera
  ;[1 1 1] Rotation of the text tip in the direction of the player's camera
  (if (Variables|Default|GetIsLookAtPlayerCamera)
    (bind _characterinbox (Variables|Default|GetCharacterInBox)
      (:then
        (bind _asbp_third_person_character (Utilities|Casting|CastToBP_ThirdPersonCharacter _characterinbox))
        (LocalVariables|SetL_CameraLocation (Transformation|GetWorldLocation (Variables|/Game/Blueprints/Characters/BP_ThirdPersonCharacter.BP_ThirdPersonCharacter_C|GetFollowCamera _asbp_third_person_character)))
        (Transformation|SetWorldRotation (Variables|Default|GetTooltipText) (Math|Rotator|FindLookatRotation (Transformation|GetWorldLocation (Variables|Default|GetTooltipText)) (LocalVariables|GetL_CameraLocation)) false false))
      (:else))))