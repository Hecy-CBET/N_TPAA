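; BP_TriggerBase is a trigger actor with a box collision volume, apparently meant as a base for environment triggers.
; The construction script sizes the box from BoxExtent and raises it by the Z extent, so its bottom sits at the box's parent origin.
; Begin overlap stores the other actor in OverlappedActor, and Interact simply returns false.
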(event Collision|EventActorBeginOverlap
  (params (OtherActor :type Actor%20Object%20Reference))
  ;[1 1 1] Save the actor when crossing it
  (Variables|Default|SetOverlappedActor OtherActor))

(fn ConstructionScript
  (Components|Box|SetBoxExtent (Variables|Default|GetBoxCollision) (Variables|Default|GetBoxExtent) true)
  (Transformation|SetRelativeLocation (Variables|Default|GetBoxCollision) (Math|Vector|MakeVector 0.0 0.0 (.Z (Math|Vector|BreakVector (Variables|Default|GetBoxExtent)))) false false))

(fn Interact
  (return false))